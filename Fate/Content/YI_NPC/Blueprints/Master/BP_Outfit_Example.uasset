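; BP_Outfit_Example is an example NPC outfit Blueprint that varies animation timing and body muscularity per instance.
; On BeginPlay it starts the UE5 component's animation at a random position and rolls a random Muscularity value.
; It applies that morph target to the skeletal mesh components beneath UE5.
; The Main mesh then receives a slightly reduced, clamped value of the same morph.
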(event `self.ReceiveBeginPlay`
  (`SkeletalMeshComponent.SetPosition` (`self.UE5`) (`KismetMathLibrary.RandomFloatInRange` 0.0 7.0) true)
  (set `self.MorphPosition` (`KismetMathLibrary.RandomFloatInRange` 0.0 1.0))
  (for _array_element (`SceneComponent.GetChildrenComponents` (`self.UE5`) true)
    (bind _asskeletal_mesh_component (cast `SkeletalMeshComponent` _array_element))
    (`SkeletalMeshComponent.SetMorphTarget` _asskeletal_mesh_component "Muscularity" (`self.MorphPosition`) true))
  (`SkeletalMeshComponent.SetMorphTarget` (`self.Main`) "Muscularity" (`KismetMathLibrary.FClamp` (- (`self.MorphPosition`) 0.2)) true))

(fn `UserConstructionScript`)
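; BPC_OutfitController is an actor component that builds a randomized modular outfit for BP_AI characters, individually or all at once.
; A seedable random stream drives mesh, socket, material and morph target choices.
; Mesh entries pass spawn-chance rolls and a queue-based topological sort that checks dependency tags for missing entries and cycles.
; Surviving entries become skeletal or static components attached to the "Parent"-tagged mesh, optionally sharing indices per type.
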(event `RandomizeAll`
  (bind _outactors (`GameplayStatics.GetAllActorsOfClass` "/Game/YI_NPC/Blueprints/Master/BP_AI.BP_AI_C"))
  (for _array_element _outactors
    (`self.RandomizeSelected` (`Actor.GetComponentByClass` _array_element "BPC_OutfitController_C"))))

(event `RandomizeSelected`
  (bind _randomstream (`self.RandomStream`))
  (`self.ClearMesh`)
  (`KismetMathLibrary.ResetRandomStream` _randomstream)
  (if (`self.DefineSeed`)
    (`KismetMathLibrary.SetRandomStreamSeed` _randomstream (`self.SetSeed`))
    (else
      (`KismetMathLibrary.SeedRandomStream` _randomstream)
      (set `self.SetSeed` (`KismetMathLibrary.BreakRandomStream` (`self.RandomStream`)))))
  (`|ExecutionSequence`
    (:`then_0`
      ;[1 0 0.03104] IMPORTANT - UPDATE THIS: Get Owner Blueprint, assign your blueprint
      (bind _asbp_ai (cast `/Game/YI_NPC/Blueprints/Master/BP_AI` (`self.GetOwner`)))
      (set `self.As BP Character` _asbp_ai))
    (:`then_1`
      (bind (_sortedstructures _success) (`self.TopologicalSort` (`self.MeshData`)))
      (if _success
        (`self.CreateMeshComponents` _sortedstructures)
        (for _array_element (`self.MorphTargets`)
          (bind (_morphposename _morphposemin _morphposemax) (break `/Game/YI_NPC/Blueprints/Master/Data/Struc_StaticMorphPoses` _array_element))
          (`/Game/YI_NPC/Blueprints/Master/BP_AI.SetMorphTarget` (`self.As BP Character`) (`KismetMathLibrary.RandomFloatInRangeFromStream` (`self.RandomStream`) _morphposemin _morphposemax)))))
    (:`then_3`
      (`self.SortMaterials`))))

(event `ClearMesh`
  (`/Game/YI_NPC/Blueprints/Master/BP_AI.ClearComponents` (`self.As BP Character`)))

(fn `CreateMeshComponents`
  (params (SortedStructure :type "Array of /Game/YI_NPC/Blueprints/Master/Data/Struc_OutfitController Structure"))
  (locals (TypeMaxIndex :type "Map of String to Integer") (MatchingIndex :type "Array of String") (TagMaxIndex :type "Map of String to Integer") (TypeRandomIndex :type "Map of String to Integer") (TagRandomIndex :type "Map of String to Integer"))
  (bind _tagmaxindex (`local.TagMaxIndex`))
  (bind _typemaxindex (`local.TypeMaxIndex`))
  (bind _as_bp_character (`self.As BP Character`))
  (bind _output (`|GetArrayItem` (`Actor.GetComponentsByTag` (`self.As BP Character`) "/Script/Engine.SkeletalMeshComponent" "Parent")))
  ;[1 1 1] Check and set parent mesh
  (`/Engine/EditorBlueprintResources/StandardMacros.IsValid` _output
    (:`Is Valid`
      (`SkinnedMeshComponent.SetSkinnedAssetAndUpdate` _output (`self.ParentMesh`) true)
      (`SkinnedMeshComponent.SetPhysicsAsset` _output (`self.ParentPhysicsAsset`) false)
      (`SkeletalMeshComponent.SetAnimInstanceClass` _output (`self.ParentAnimationBlueprint`))
      (`|ExecutionSequence`
        (:`then_0`
          (`|ExecutionSequence`
            (:`then_0`
              (for _array_element SortedStructure
                (if (`self.SameTypesMustMatchRandomIndex`)
                  (bind (_animationblueprint _spawnchance _type _uniquetag _dependenttag _skeletalmesh _staticmesh) (break `/Game/YI_NPC/Blueprints/Master/Data/Struc_OutfitController` _array_element))
                  (`BlueprintMapLibrary.Map_Add` (`local.TagMaxIndex`) _uniquetag)
                  (bind (_value _returnvalue) (`BlueprintMapLibrary.Map_Find` (`local.TypeMaxIndex`) _type))
                  (if _returnvalue
                    (bind _returnvalue_2 (- (`KismetArrayLibrary.Array_Length` _skeletalmesh) 1))
                    (bind _returnvalue_3 (- (`KismetArrayLibrary.Array_Length` _staticmesh) 1))
                    (if (or (== _value _returnvalue_2) (== _value _returnvalue_3))
                      (`BlueprintMapLibrary.Map_Add` (`local.TypeMaxIndex`) _type (select `bool` (> _returnvalue_2 _returnvalue_3) :`false` _returnvalue_3 :`true` _returnvalue_2) :!label _label)
                      (else
                        (`|ExecutionSequence`
                          (:`then_0`
                            (if (and (`KismetArrayLibrary.Array_IsNotEmpty` _skeletalmesh) (< _returnvalue_2 _value))
                              (`BlueprintMapLibrary.Map_Add` (`local.TypeMaxIndex`) _type _returnvalue_2)
                              (elif (and (`KismetArrayLibrary.Array_IsNotEmpty` _staticmesh) (< _returnvalue_3 0))
                                (`BlueprintMapLibrary.Map_Add` (`local.TypeMaxIndex`) _type _returnvalue_3)
                                (else
                                  (`KismetSystemLibrary.PrintString` (`KismetStringLibrary.Concat_StrStr` "Error: No meshes found on unique tag item `" _uniquetag "`. Please check the data structure.") true true (struct :`R` 0.901042 :`G` 0.043346 :`A` 1.0) 10.0)
                                  (return))))
                            (`self.EnableDebugCheck`)
                            (`KismetSystemLibrary.PrintString` (`KismetStringLibrary.Concat_StrStr` "Warning: Matching types `" _type "` array size does not match. Unless this is intentional, it may cause matching issues. Index range reduced, to prevent out of bounds errors.") true true (struct :`R` 0.901042 :`G` 0.043346 :`A` 1.0) 10.0)))))
                    (else
                      (goto _label)))
                  (else
                    (bind (_success _isskeletal _lastindex) (`self.CheckMeshInput` _skeletalmesh _staticmesh))
                    (if _success
                      (`BlueprintMapLibrary.Map_Add` (`local.TagMaxIndex`) _uniquetag _lastindex))))))
            (:`then_1`
              (if (`self.SameTypesMustMatchRandomIndex`)
                (bind _keys (`BlueprintMapLibrary.Map_Keys` _typemaxindex))
                (for _array_element_2 _keys
                  (`BlueprintMapLibrary.Map_Add` (`local.TypeRandomIndex`) _array_element_2 (`KismetMathLibrary.RandomIntegerFromStream` (`self.RandomStream`) (- (`BlueprintMapLibrary.Map_Find` _typemaxindex _array_element_2) 1))))
                (for _array_element_3 (`self.MeshData`)
                  (bind (_animationblueprint_2 _spawnchance_2 _type_2 _uniquetag_2) (break `/Game/YI_NPC/Blueprints/Master/Data/Struc_OutfitController` _array_element_3))
                  (`BlueprintMapLibrary.Map_Add` (`local.TagRandomIndex`) _uniquetag_2 (`BlueprintMapLibrary.Map_Find` (`local.TypeRandomIndex`) _type_2)))
                (else
                  (bind _keys_2 (`BlueprintMapLibrary.Map_Keys` _tagmaxindex))
                  (for _array_element_4 _keys_2
                    (`BlueprintMapLibrary.Map_Add` (`local.TagRandomIndex`) _array_element_4 (`KismetMathLibrary.RandomIntegerFromStream` (`self.RandomStream`) (- (`BlueprintMapLibrary.Map_Find` _tagmaxindex _array_element_4) 1)))))))))
        (:`then_1`
          (for _array_element_5 SortedStructure
            (bind (_animationblueprint_3 _spawnchance_3 _type_3 _uniquetag_3 _dependenttag_2 _skeletalmesh_2 _staticmesh_2 _optionalphysicsasset _optionalsocketname _optionalsocketitemtransformoffset) (break `/Game/YI_NPC/Blueprints/Master/Data/Struc_OutfitController` _array_element_5))
            (bind _returnvalue_4 (`KismetArrayLibrary.Array_IsNotEmpty` _skeletalmesh_2))
            (if (and _returnvalue_4 (`KismetArrayLibrary.Array_IsNotEmpty` _staticmesh_2))
              (`self.EnableDebugCheck`)
              (`KismetSystemLibrary.PrintString` (`KismetStringLibrary.Concat_StrStr` "Error: You have assigned a static mesh, and a skeletal mesh, to the same mesh type `" _uniquetag_3 "` . \n \nPlease seperate these into new types, or remove the meshes."))
              (elif _returnvalue_4
                (bind _returnvalue_5 (`|AddComponentByClass` :`self` _as_bp_character :`Class` "/Script/Engine.SkeletalMeshComponent"))
                (bind (_outitem _outindex) (`KismetArrayLibrary.Array_RandomFromStream` _optionalsocketname (`self.RandomStream`)))
                (bind _returnvalue_6 (`KismetStringLibrary.Conv_StringToName` _outitem))
                (`SceneComponent.K2_AttachToComponent` _returnvalue_5 _output _returnvalue_6 "KeepRelative" "KeepRelative" "KeepRelative" true)
                (set `SceneComponent.bUseAttachParentBound` true _returnvalue_5)
                (bind _value_2 (`BlueprintMapLibrary.Map_Find` (`local.TagRandomIndex`) _uniquetag_3))
                (`SkinnedMeshComponent.SetSkinnedAssetAndUpdate` _returnvalue_5 (`|GetArrayItem` _skeletalmesh_2 _value_2) true)
                (`KismetArrayLibrary.Array_Add` (`ActorComponent.ComponentTags` _returnvalue_5) "OutfitController")
                (bind _output_2 (`|GetArrayItem` _optionalsocketitemtransformoffset _outindex))
                (`SceneComponent.K2_SetRelativeTransform` _returnvalue_5 _output_2 false false)
                (`/Engine/EditorBlueprintResources/StandardMacros.IsValid` _optionalphysicsasset
                  (:`Is Valid`
                    (`SkinnedMeshComponent.SetPhysicsAsset` _returnvalue_5 _optionalphysicsasset false))
                  (:`Is Not Valid`
                    _))
                (if (`KismetSystemLibrary.IsValidClass` _animationblueprint_3)
                  (`SkeletalMeshComponent.SetAnimInstanceClass` _returnvalue_5 _animationblueprint_3))
                (else
                  (bind _returnvalue_7 (`|AddComponentByClass` :`self` _as_bp_character :`Class` "/Script/Engine.StaticMeshComponent"))
                  (`SceneComponent.K2_AttachToComponent` _returnvalue_7 _output _returnvalue_6 "KeepRelative" "KeepRelative" "KeepRelative" true)
                  (set `SceneComponent.bUseAttachParentBound` true _returnvalue_7)
                  (`KismetArrayLibrary.Array_Add` (`ActorComponent.ComponentTags` _returnvalue_7) "OutfitController")
                  (`SceneComponent.K2_SetRelativeTransform` _returnvalue_7 _output_2 false false)
                  (`StaticMeshComponent.SetStaticMesh` _returnvalue_7 (`|GetArrayItem` _staticmesh_2 _value_2)))))))))
    (:`Is Not Valid`
      (`self.EnableDebugCheck`)
      (`KismetSystemLibrary.PrintString` "Error: Parent Skeletal Mesh component not detected. This must be setup manually. \n \nPlease make sure a skeletal mesh component, with the tag \"Parent\", has been assigned in your blueprint component list."))))

(fn `DestroyComponents`
  (locals (SkeletalMeshes :type "Array of SkeletalMeshComponent Object Reference") (StaticMeshes :type "Array of StaticMeshComponent Object Reference"))
  (bind _as_bp_character (`self.As BP Character`))
  (`|ExecutionSequence`
    (:`then_0`
      (set `local.SkeletalMeshes` (`Actor.GetComponentsByTag` _as_bp_character "/Script/Engine.SkeletalMeshComponent" "OutfitController"))
      (for _array_element (`local.SkeletalMeshes`)
        (`/Engine/EditorBlueprintResources/StandardMacros.IsValid` _array_element
          (:`Is Valid`
            (`self.K2_DestroyComponent` _array_element)))))
    (:`then_1`
      (set `local.StaticMeshes` (`Actor.GetComponentsByTag` _as_bp_character "/Script/Engine.StaticMeshComponent" "OutfitController"))
      (for _array_element_2 (`local.StaticMeshes`)
        (`/Engine/EditorBlueprintResources/StandardMacros.IsValid` _array_element_2
          (:`Is Valid`
            (`self.K2_DestroyComponent` _array_element_2)))))
    (:`then_2`
      (set `local.SkeletalMeshes` (`Actor.GetComponentsByTag` _as_bp_character "/Script/Engine.SkeletalMeshComponent" "Parent"))
      (for _array_element_3 (`local.SkeletalMeshes`)
        (`SkinnedMeshComponent.SetSkinnedAssetAndUpdate` _array_element_3 null true)))))

(fn `MatchRandomIndexByType`
  (params (OrderedStructure :type "Array of /Game/YI_NPC/Blueprints/Master/Data/Struc_OutfitController Structure"))
  (locals (Types :type Boolean))
  (for _ OrderedStructure
    _))

(fn `RandomFloatArray`
  (params (Min :type "Float (double-precision)") (Max :type "Float (double-precision)") (ArraySize :type Integer))
  (returns (NewParam :type "Array of Float (double-precision)"))
  (locals (Floats :type "Array of Float (double-precision)"))
  (bind _floats (`local.Floats`))
  (`KismetArrayLibrary.Array_Clear` _floats)
  (for _ (range (+ ArraySize 1))
    (`KismetArrayLibrary.Array_Add` _floats (`self.RandomFloat` Min Max)))
  (return (`local.Floats`)))

(fn `SortMaterials`
  (locals (Instances :type "Array of MaterialInstance Object Reference") (MaterialTypes :type "Array of String") (MaterialIndexes :type "Array of Integer") (SlotNames :type "Array of String"))
  (bind _materialtypes (`local.MaterialTypes`))
  (`|ExecutionSequence`
    (:`then_0`
      (for _array_element (`self.Material Options`)
        (bind (_slotname _type _materialinstances) (break `/Game/YI_NPC/Blueprints/Master/Data/Struc_MaterialOptions` _array_element))
        (if (not (`KismetArrayLibrary.Array_Contains` _materialtypes _type))
          (`KismetArrayLibrary.Array_Add` _materialtypes _type)
          (`KismetArrayLibrary.Array_Add` (`local.MaterialIndexes`) (`.OutIndex` (`KismetArrayLibrary.Array_RandomFromStream` _materialinstances (`self.RandomStream`)))))))
    (:`then_1`
      (for _array_element_2 (`self.Material Options`)
        (bind (_slotname_2 _type_2 _materialinstances_2) (break `/Game/YI_NPC/Blueprints/Master/Data/Struc_MaterialOptions` _array_element_2))
        (`KismetArrayLibrary.Array_Add` (`local.SlotNames`) _slotname_2)
        (`KismetArrayLibrary.Array_Add` (`local.Instances`) (`|GetArrayItem` _materialinstances_2 (`|GetArrayItem` (`local.MaterialIndexes`) (`KismetArrayLibrary.Array_Find` (`local.MaterialTypes`) _type_2))))))
    (:`then_2`
      (`/Game/YI_NPC/Blueprints/Master/BP_AI.SetMaterials` (`self.As BP Character`) (`local.SlotNames`) (`local.Instances`)))))

(fn `TopologicalSort`
  (params (Structures :type "Array of /Game/YI_NPC/Blueprints/Master/Data/Struc_OutfitController Structure"))
  (returns (SortedStructures :type "Array of /Game/YI_NPC/Blueprints/Master/Data/Struc_OutfitController Structure") (Success :type Boolean))
  (locals (StructureMap :type "Map of String to /Game/YI_NPC/Blueprints/Master/Data/Struc_OutfitController Structure") (IncomingEdges :type "Map of String to Object Object Reference") (Queue :type "Array of String") (Sorted :type "Array of /Game/YI_NPC/Blueprints/Master/Data/Struc_OutfitController Structure") (CurrentQueueItem :type String) (SpawnedTags :type "Map of String to Boolean"))
  (bind _queue (`local.Queue`))
  (bind _incomingedges (`local.IncomingEdges`))
  (bind _incomingedges_2 (`local.IncomingEdges`))
  (bind _incomingedges_3 (`local.IncomingEdges`))
  (bind _incomingedges_4 (`local.IncomingEdges`))
  (`|ExecutionSequence`
    (:`then_0`
      ;[1 1 1] Add base map entry key's for reference
      (for (_array_element _array_index) Structures
        (bind (_animationblueprint _spawnchance _type _uniquetag) (break `/Game/YI_NPC/Blueprints/Master/Data/Struc_OutfitController` _array_element))
        (if (not (`.ReturnValue` (`BlueprintMapLibrary.Map_Find` (`local.IncomingEdges`) _uniquetag)))
          (`BlueprintMapLibrary.Map_Add` (`local.StructureMap`) _uniquetag _array_element)
          (`BlueprintMapLibrary.Map_Add` (`local.IncomingEdges`) _uniquetag)
          (else
            (`KismetSystemLibrary.PrintString` (`KismetStringLibrary.Concat_StrStr` "Error: Mesh tag duplicate found at index `" (`KismetStringLibrary.Conv_IntToString` _array_index) "` of the mesh data structure. Please make sure tags are unique, and then try again.") true true (struct :`R` 0.901042 :`G` 0.043346 :`A` 1.0) 10.0)
            (return _ false)))))
    (:`then_1`
      ;[1 1 1] Check mapped incoming edges, for any dependent tags that aren't present. If they exist, throw an error message and stop to prevent an infinite loop
      (for _array_element_2 Structures
        (bind (_animationblueprint_2 _spawnchance_2 _type_2 _uniquetag_2 _dependenttag) (break `/Game/YI_NPC/Blueprints/Master/Data/Struc_OutfitController` _array_element_2))
        (for _array_element_3 _dependenttag
          (if (not (`.ReturnValue` (`BlueprintMapLibrary.Map_Find` (`local.IncomingEdges`) _array_element_3)))
            (`KismetSystemLibrary.PrintString` (`KismetStringLibrary.Concat_StrStr` "Error: Dependent tag  `" _array_element_3 "` does not exist as a mesh type. \n" "Structure: \"" _uniquetag_2 "\"") true true (struct :`R` 0.901042 :`G` 0.043346 :`A` 1.0) 10.0)
            (return _ false)))))
    (:`then_2`
      ;[1 1 1] Foreach structure/mesh type, iterate through it's dependent types (if they exist). If there are dependent tags, increase the incoming edges by one, for the dependent mesh referenced by this tag.
      (for _array_element_4 Structures
        (bind (_animationblueprint_3 _spawnchance_3 _type_3 _uniquetag_3 _dependenttag_2) (break `/Game/YI_NPC/Blueprints/Master/Data/Struc_OutfitController` _array_element_4))
        (if (`KismetArrayLibrary.Array_IsNotEmpty` _dependenttag_2)
          (for _array_element_5 _dependenttag_2
            (bind (_value _returnvalue) (`BlueprintMapLibrary.Map_Find` _incomingedges_3 _array_element_5))
            (if _returnvalue
              (`BlueprintMapLibrary.Map_Add` _incomingedges_3 _array_element_5 (+ _value 1))))))
      (`self.EnableDebugCheck`)
      (for _array_element_6 Structures
        (bind (_animationblueprint_4 _spawnchance_4 _type_4 _uniquetag_4) (break `/Game/YI_NPC/Blueprints/Master/Data/Struc_OutfitController` _array_element_6))
        (`KismetSystemLibrary.PrintString` (`KismetStringLibrary.Concat_StrStr` "Structure Type `" _uniquetag_4 "` has `" (`KismetStringLibrary.Conv_IntToString` (`BlueprintMapLibrary.Map_Find` _incomingedges_3 _uniquetag_4)) "` incoming edges.") true true (struct :`R` 0.291353 :`G` 1.0 :`B` 0.08707 :`A` 1.0) 10.0)))
    (:`then_3`
      ;[1 1 1] Foreach incoming edge key, if the value is zero, assign it to the queue
      (bind _keys (`BlueprintMapLibrary.Map_Keys` _incomingedges_4))
      (for _array_element_7 _keys
        (if (== (`BlueprintMapLibrary.Map_Find` _incomingedges_4 _array_element_7) 0)
          (`KismetArrayLibrary.Array_Add` (`local.Queue`) _array_element_7)
          (`self.EnableDebugCheck`)
          (`KismetSystemLibrary.PrintString` (`KismetStringLibrary.Concat_StrStr` "Adding `" _array_element_7 "` to queue. No edges detected.") true true (struct :`R` 0.370761 :`G` 1.0 :`B` 0.930213 :`A` 1.0) 10.0))))
    (:`then_4`
      ;[1 1 1] This block handles the sorting of the assigned structures and maps, based on dependency tags and mesh types
      ;;[1 1 1] While the queue is not empty, get the first item of the queue to process, then remove it from the queue.
      (while (`KismetArrayLibrary.Array_IsNotEmpty` _queue)
        (bind _output_get (set `local.CurrentQueueItem` (`|GetArrayItem` _queue)))
        (`KismetArrayLibrary.Array_Remove` _queue)
        (bind (_value_2 _returnvalue_2) (`BlueprintMapLibrary.Map_Find` (`local.SpawnedTags`) _output_get))
        (if (not (and _value_2 _returnvalue_2))
          (`|ExecutionSequence`
            (:`then_0`
              (bind _value_3 (`BlueprintMapLibrary.Map_Find` (`local.StructureMap`) _output_get))
              (bind (_animationblueprint_5 _spawnchance_5 _type_5 _uniquetag_5 _dependenttag_3) (break `/Game/YI_NPC/Blueprints/Master/Data/Struc_OutfitController` _value_3))
              ;;[1 1 1] Check if the mesh type passes it's spawn check, assign the mesh type to the spawned tag map, and set is to true/false.
              (if (>= _spawnchance_5 (`KismetMathLibrary.RandomFloatFromStream` (`self.RandomStream`)))
                (`BlueprintMapLibrary.Map_Add` (`local.SpawnedTags`) _uniquetag_5 true)
                (else
                  (`BlueprintMapLibrary.Map_Add` (`local.SpawnedTags`) _uniquetag_5))))
            (:`then_1`
              ;;[1 1 1] Check the queued items incoming edge count. If it's greater than 0, --1, if it equals 0, add it back to the queue as all dependencies have been checked. This ensures it will be processed into the sort order, after spawned tag validation is done.
              (for _array_element_8 _dependenttag_3
                (bind _value_4 (`BlueprintMapLibrary.Map_Find` _incomingedges _array_element_8))
                (if (> _value_4 0)
                  (bind _returnvalue_3 (- _value_4 1))
                  (`BlueprintMapLibrary.Map_Add` _incomingedges _array_element_8 _returnvalue_3)
                  (if (== _returnvalue_3 -1)
                    (`KismetArrayLibrary.Array_Add` (`local.Queue`) _array_element_8)
                    (`self.EnableDebugCheck`)
                    (`KismetSystemLibrary.PrintString` (`KismetStringLibrary.Concat_StrStr` "Type `" _array_element_8 "` now has `0` incoming edges. Adding to queue . . .") true true (struct :`R` 1.0 :`B` 0.756678 :`A` 1.0) 10.0)))))
            (:`then_2`
              ;;[1 1 1] If there are dependent tags, check the spawned tags map, to make sure these dependencies have been spawned. If there are no dependent tags, or the dependencies have been spawned, add them to the sorted array.
              (if (`KismetArrayLibrary.Array_IsEmpty` _dependenttag_3)
                (if (`BlueprintMapLibrary.Map_Find` (`local.SpawnedTags`) _uniquetag_5)
                  (`KismetArrayLibrary.Array_Add` (`local.Sorted`) _value_3 :!label _label))
                (else
                  (for _array_element_9 _dependenttag_3
                    (bind (_value_5 _returnvalue_4) (`BlueprintMapLibrary.Map_Find` (`local.SpawnedTags`) _array_element_9))
                    (if _returnvalue_4
                      (if _value_5
                        (goto _label)
                        (else
                          (`self.EnableDebugCheck`)
                          (`KismetSystemLibrary.PrintString` (`KismetStringLibrary.Concat_StrStr` "Dependent Type `" _array_element_9 "` failed it's spawn chance. \n" "Mesh type `" _uniquetag_5 "` will not be spawned.") true true (struct :`R` 1.0 :`G` 0.506724 :`A` 1.0) 10.0)))
                      (else
                        (`KismetArrayLibrary.Array_Add` (`local.Queue`) _uniquetag_5))))))))))
      ;;[1 1 1] If incoming edges is 0 for all keys, output the sorted array, otherwise, a circuler dependency loop has been detected, no output is possible, infinite loop avoided
      (bind _keys_2 (`BlueprintMapLibrary.Map_Keys` _incomingedges_2))
      (for _array_element_10 _keys_2
        (`|ExecutionSequence`
          (:`then_0`
            (`self.EnableDebugCheck`)
            (bind _value_6 (`BlueprintMapLibrary.Map_Find` _incomingedges_2 _array_element_10))
            (`KismetSystemLibrary.PrintString` (`KismetStringLibrary.Concat_StrStr` "Final Edges of Type `" _array_element_10 "` = `" (`KismetStringLibrary.Conv_IntToString` _value_6) "`") true true (struct :`R` 0.053933 :`G` 1.0 :`A` 1.0) 10.0))
          (:`then_1`
            (if (> _value_6 0)
              (`|ExecutionSequence`
                (:`then_0`
                  (`self.EnableDebugCheck`)
                  (`KismetSystemLibrary.PrintString` "E.g. if the hand relies on the arm, and the arm relies on the body, the hand should have dependent tags for the hand and body." true true (struct :`R` 1.0 :`G` 0.035793 :`A` 1.0) 10.0)
                  (`KismetSystemLibrary.PrintString` "Error: Cyclical dependency loop detected. If you are referencing complex dependencies, make sure to reference all dependencies in the chain. " true true (struct :`R` 1.0 :`G` 0.035793 :`A` 1.0) 10.0))
                (:`then_1`
                  (return _ false)))))))
      (`|ExecutionSequence`
        (:`then_0`
          (if true
            (`self.EnableDebugCheck`)
            (for _array_element_11 _
              (`KismetSystemLibrary.PrintString` (`KismetStringLibrary.Concat_StrStr` "Final Type List: " (`.UniqueTag_109_2005F1EC44EAA376E4FCB1B5AB693251` (break `/Game/YI_NPC/Blueprints/Master/Data/Struc_OutfitController` _array_element_11))) true true (struct :`G` 1.0 :`B` 0.464896 :`A` 1.0) 10.0))))
        (:`then_1`
          (return (`local.Sorted`) true))))))